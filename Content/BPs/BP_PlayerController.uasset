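; Player controller that turns Enhanced Input actions into movement, camera rotation and jumping for BP_Character.
; On possess it caches the character and adds the input mapping context.
; Move and camera input forward directly to the character, while jump checks CanJump, then calls Jump and SetGravityScale(true) for a custom fall speed.
; A disconnected branch holding SetGravityScale(false) and a DoOnce reset never runs.
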(event Input|EnhancedActionEvents|EnhancedInputActionIA_Move
  (params (ActionValue :type Vector%202D%20Structure) (ElapsedSeconds :type Float%20%28double-precision%29) (TriggeredSeconds :type Float%20%28double-precision%29) (InputAction :type Input%20Action%20Object%20Reference :default "/Game/Input/IA_Move.IA_Move"))
  ;[1 1 1] Move
  (Default|CharacterMove (Variables|Default|GetBP%20Character) (Math|Vector|MakeVector (.x ActionValue) (.y ActionValue) 0.0)))

(event Input|EnhancedActionEvents|EnhancedInputActionIA_CamRotation
  (params (ActionValue :type Vector%202D%20Structure) (ElapsedSeconds :type Float%20%28double-precision%29) (TriggeredSeconds :type Float%20%28double-precision%29) (InputAction :type Input%20Action%20Object%20Reference :default "/Game/Input/IA_CamRotation.IA_CamRotation"))
  (bind _bp_character (Variables|Default|GetBP%20Character))
  (Pawn|Input|AddControllerYawInput _bp_character (.x ActionValue))
  (Pawn|Input|AddControllerPitchInput _bp_character (.y ActionValue)))

(event Input|EnhancedActionEvents|EnhancedInputActionIA_Jump
  (params (ActionValue :type Boolean) (ElapsedSeconds :type Float%20%28double-precision%29) (TriggeredSeconds :type Float%20%28double-precision%29) (InputAction :type Input%20Action%20Object%20Reference :default "/Game/Input/IA_Jump.IA_Jump"))
  (bind _bp_character (Variables|Default|GetBP%20Character))
  (if (Character|CanJump (Variables|Default|GetBP%20Character))
    (Character|Jump _bp_character)
    (Default|SetGravityScale _bp_character true)))

(event EventPossess
  (params (PossessedPawn :type Pawn%20Object%20Reference))
  (bind _asbp_character (Utilities|Casting|CastToBP_Character PossessedPawn))
  (Variables|Default|SetBP%20Character _asbp_character)
  (Input|AddMappingContext (PlayerController|LocalPlayerSubsystems|GetEnhancedInputLocalPlayerSubsystem) "/Game/Input/IMC.IMC" 0 "(bIgnoreAllPressedKeysUntilRelease=True,bForceImmediately=False,bNotifyUserSettings=False)"))

(fn ConstructionScript)