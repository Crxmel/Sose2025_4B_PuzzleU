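; Player character with camera-relative movement, mouse look, custom jump/fall gravity scales, and contact damage to health components it hits.
; Interact drops any held item, otherwise sphere-traces from the camera to message interface actors or collect BP_PickupActors.
; Pickups form an array that can be cycled, hidden or dropped, and interactions can consume the current one.
; A separately held item toggles between back and front attach points, where mouse input rotates it for inspection.
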(event Custom|Character_Move
  (params (Local%20Direction :type Vector))
  (Pawn|Input|AddMovementInput (Math|Transform|TransformDirection (Math|Transform|MakeTransform "0, 0, 0" (Math|Rotator|MakeRotator 0.0 0.0 (.yaw (Transformation|GetWorldRotation (Variables|Default|GetCamera)))) "1.000000,1.000000,1.000000") Local%20Direction) 1.0 false))

(event Custom|SetGravityScale
  (params (IsJumping :type Boolean))
  (Variables|/Script/Engine.CharacterMovementComponent|SetGravityScale (Variables|Character|GetCharacterMovement) (Math|Float|SelectFloat (Variables|Default|GetGravetyScale_Jump) (Variables|Default|GetgravetyScale_Fall) IsJumping)))

(event Custom|Pichup
  (params (static%20mesh :type Static%20Mesh%20Component%20Object%20Reference) (Target :type Actor%20Object%20Reference))
  ;[0.15 0.15 0.15 0.5] ItemInHand
  (Variables|Default|SetItemInHand static%20mesh)
  (Transformation|AttachComponentToComponent Target (Variables|Default|GetGegenstandBack) "None" "SnapToTarget" "SnapToTarget" "KeepWorld" true)
  (Physics|SetSimulatePhysics (Variables|Default|GetItemInHand) false))

(event Custom|Drop%20item
  ;[0.15 0.15 0.15 0.5] ItemInHand
  (Transformation|DetachFromActor (stale Custom|Pichup Target) "KeepWorld" "KeepWorld" "KeepWorld")
  (Physics|SetSimulatePhysics (Variables|Default|GetItemInHand) true))

(event Custom|Set%20rotation%20in%20hand
  (params (X :type Float%20%28double-precision%29) (Y :type Float%20%28double-precision%29))
  ;[0.15 0.15 0.15 0.5] ItemInHand
  (CallFunction|RotatonItem X Y))

(event Custom|WatchItem
  ;[0.15 0.15 0.15 0.5] ItemInHand
  (if (Variables|Default|GetShift%20Pressed)
    (Transformation|AttachComponentToComponent (stale Custom|Pichup Target) (Variables|Default|GetGegenstandFront) "None" "SnapToTarget" "SnapToTarget" "KeepWorld" true)
    (else
      (Transformation|AttachComponentToComponent (stale Custom|Pichup Target) (Variables|Default|GetGegenstandBack) "None" "SnapToTarget" "SnapToTarget" "KeepWorld" true))))

(event Input|EnhancedActionEvents|EnhancedInputActionIA_Move
  (params (ActionValue :type Vector%202D%20Structure) (ElapsedSeconds :type Float%20%28double-precision%29) (TriggeredSeconds :type Float%20%28double-precision%29) (InputAction :type Input%20Action%20Object%20Reference :default "/Game/Input/IA/IA_Move.IA_Move"))
  ;[1 1 1] MoveInput
  (CallFunction|CharacterMove (Math|Vector|MakeVector (.x ActionValue) (.y ActionValue) 0.0)))

(event Input|EnhancedActionEvents|EnhancedInputActionIA_Mous
  (params (ActionValue :type Vector%202D%20Structure) (ElapsedSeconds :type Float%20%28double-precision%29) (TriggeredSeconds :type Float%20%28double-precision%29) (InputAction :type Input%20Action%20Object%20Reference :default "/Game/Input/IA/IA_Mous.IA_Mous"))
  ;[0.15 0.15 0.15 0.5] CamRotation
  (if (Variables|Default|GetShift%20Pressed)
    (CallFunction|SetRotationinHand (.x ActionValue) (.y ActionValue))
    (else
      (Pawn|Input|AddControllerYawInput (.x ActionValue))
      (Pawn|Input|AddControllerPitchInput (.y ActionValue)))))

(event Input|EnhancedActionEvents|EnhancedInputActionIA_Jump
  (params (ActionValue :type Boolean) (ElapsedSeconds :type Float%20%28double-precision%29) (TriggeredSeconds :type Float%20%28double-precision%29) (InputAction :type Input%20Action%20Object%20Reference :default "/Game/Input/IA/IA_Jump.IA_Jump"))
  ;[0.15 0.15 0.15 0.5] JumpInput
  (if (Character|CanJump)
    (Character|Jump)
    (CallFunction|SetGravityScale true)))

(event Input|EnhancedActionEvents|EnhancedInputActionIA_Interact
  (params (ActionValue :type Boolean) (ElapsedSeconds :type Float%20%28double-precision%29) (TriggeredSeconds :type Float%20%28double-precision%29) (InputAction :type Input%20Action%20Object%20Reference :default "/Game/Input/IA_Interact.IA_Interact"))
  ;[0.15 0.15 0.15 0.5] für item in hand
  (Utilities|IsValid (Variables|Default|GetItemInHand)
    (:Is%20Valid
      (CallFunction|DropItem)
      (Variables|Default|SetItemInHand 0)
      (Variables|Default|SetShift%20Pressed false))
    (:Is%20Not%20Valid
      (CallFunction|TryInteract))))

(event Input|EnhancedActionEvents|EnhancedInputActionIA_Shift
  (params (ActionValue :type Boolean) (ElapsedSeconds :type Float%20%28double-precision%29) (TriggeredSeconds :type Float%20%28double-precision%29) (InputAction :type Input%20Action%20Object%20Reference :default "/Game/Input/IA/IA_Shift.IA_Shift"))
  (Utilities|IsValid (Variables|Default|GetItemInHand)
    (:Is%20Valid
      (Variables|Default|SetShift%20Pressed (not (Variables|Default|GetShift%20Pressed)))
      (CallFunction|WatchItem))))

(event Input|EnhancedActionEvents|EnhancedInputActionIA_DropPickup
  (params (ActionValue :type Boolean) (ElapsedSeconds :type Float%20%28double-precision%29) (TriggeredSeconds :type Float%20%28double-precision%29) (InputAction :type Input%20Action%20Object%20Reference :default "/Game/Input/IA_DropPickup.IA_DropPickup"))
  (bind _pickup (CallFunction|GetCurrentpickup))
  (Utilities|IsValid _pickup
    (:Is%20Valid
      (Default|Drop _pickup)
      (CallFunction|RemouvecurrendPickup))))

(event Input|EnhancedActionEvents|EnhancedInputActionIA_ToglePickupVisibility
  (params (ActionValue :type Boolean) (ElapsedSeconds :type Float%20%28double-precision%29) (TriggeredSeconds :type Float%20%28double-precision%29) (InputAction :type Input%20Action%20Object%20Reference :default "/Game/Input/IA_ToglePickupVisibility.IA_ToglePickupVisibility"))
  (CallFunction|Stasch/UnstastPickup (not (Variables|Default|GetIsPickupStash?))))

(event Input|EnhancedActionEvents|EnhancedInputActionIA_NextPickup
  (params (ActionValue :type Boolean) (ElapsedSeconds :type Float%20%28double-precision%29) (TriggeredSeconds :type Float%20%28double-precision%29) (InputAction :type Input%20Action%20Object%20Reference :default "/Game/Input/IA_NextPickup.IA_NextPickup"))
  (CallFunction|SelectPickup true))

(event Input|EnhancedActionEvents|EnhancedInputActionIA_PriviosPickup
  (params (ActionValue :type Boolean) (ElapsedSeconds :type Float%20%28double-precision%29) (TriggeredSeconds :type Float%20%28double-precision%29) (InputAction :type Input%20Action%20Object%20Reference :default "/Game/Input/IA_PriviosPickup.IA_PriviosPickup"))
  (CallFunction|SelectPickup false))

(event Collision|EventHit
  (params (MyComp :type Primitive%20Component%20Object%20Reference) (Other :type Actor%20Object%20Reference) (OtherComp :type Primitive%20Component%20Object%20Reference) (bSelfMoved :type Boolean) (HitLocation :type Vector :default "0, 0, 0") (HitNormal :type Vector :default "0, 0, 0") (NormalImpulse :type Vector :default "0, 0, 0") (Hit :type Hit%20Result%20Structure%20%28by%20ref%29))
  (bind _returnvalue (Actor|GetComponentbyClass Other "/Game/BPs/healthSystem/BP_HealthComponent.BP_HealthComponent_C"))
  (Utilities|IsValid _returnvalue
    (:Is%20Valid
      (Default|TakeDamage _returnvalue (Variables|Default|GetContactDamage)))))

(event EventTick
  (params (DeltaSeconds :type Float%20%28single-precision%29))
  ;[1 1 1] Für custom fallgeschwindichkeit
  (if (>= (.z (Variables|/Script/Engine.MovementComponent|GetVelocity (Variables|Character|GetCharacterMovement))) 0.0)
    (CallFunction|SetGravityScale false)))

(fn ConstructionScript)

(fn TryInteract
  (bind _camera (Variables|Default|GetCamera))
  (bind _returnvalue (Transformation|GetWorldLocation _camera))
  (bind (_outhit _returnvalue_2) (Collision|SphereTraceForObjects _returnvalue (+ _returnvalue (* (Math|Vector|GetForwardVector _camera) (Variables|Default|GetMaxInteractionRange))) 3.0 (Utilities|Array|MakeArray "ObjectTypeQuery1" "ObjectTypeQuery2" "ObjectTypeQuery3" "ObjectTypeQuery4") false 0 "Persistent"))
  (if _returnvalue_2
    (if (Utilities|DoesObjectImplementInterface (.HitActor (Collision|BreakHitResult _outhit)) "/Game/BPs/KeyPats/BP_interactionInterface.BP_interactionInterface_C")
      (bind _used_up_pickup (Class|BPInteractionInterface|Interact(Message) (.HitActor (Collision|BreakHitResult _outhit)) self (select (Variables|Default|GetIsPickupStash?) 0 (CallFunction|GetCurrentpickup))))
      (if _used_up_pickup
        (CallFunction|RemouvecurrendPickup))
      (else
        (bind _asbp_pickup_actor (Utilities|Casting|CastToBP_PickupActor (.HitActor (Collision|BreakHitResult _outhit))))
        (CallFunction|Stasch/UnstastPickup true)
        (bind _returnvalue_3 (Utilities|Array|Add (Variables|Default|GetPickup/Array) _asbp_pickup_actor))
        (Variables|Default|SetPickupIndex _returnvalue_3)
        (Default|PrepareforHoldingAAttatchto _asbp_pickup_actor (Variables|Default|GetGegenstandFront))
        (CallFunction|Stasch/UnstastPickup false)))))

(fn RotatonItem
  (params (yaw :type Float%20%28double-precision%29) (pitch :type Float%20%28double-precision%29))
  (Transformation|AddWorldRotation (Variables|Default|GetGegenstandFront) (Math|Rotator|CombineRotators (Math|Vector|RotatorfromAxisandAngle "0.000000,0.000000,1.000000" (* yaw -1.0)) (Math|Vector|RotatorfromAxisandAngle (Transformation|GetActorRightVector) (* pitch -1.0))) false false))

(fn Stasch/UnstastPickup
  (params (bNewHidden :type Boolean))
  (Utilities|IsValid (CallFunction|GetCurrentpickup)
    (:Is%20Valid
      (Variables|Default|SetIsPickupStash? bNewHidden)
      (Rendering|SetActorHiddenInGame (CallFunction|GetCurrentpickup) bNewHidden))))

(fn GetCurrentpickup
  (return (Utilities|Array|Get(acopy) (Variables|Default|GetPickup/Array) (Variables|Default|GetPickupIndex))))

(fn SelectPickup
  (params (SelectNext :type Boolean))
  (CallFunction|Stasch/UnstastPickup true)
  (Variables|Default|SetPickupIndex (+ (Variables|Default|GetPickupIndex) (Math|Integer|SelectInt 1 -1 SelectNext)))
  (Utilities|FlowControl|Sequence
    (:then_0
      (if (> (Variables|Default|GetPickupIndex) (Utilities|Array|LastIndex (Variables|Default|GetPickup/Array)))
        (Variables|Default|SetPickupIndex 0)))
    (:then_1
      (if (< (Variables|Default|GetPickupIndex) 0)
        (Variables|Default|SetPickupIndex (Utilities|Array|LastIndex (Variables|Default|GetPickup/Array)))))
    (:then_2
      (CallFunction|Stasch/UnstastPickup false))))

(fn RemouvecurrendPickup
  (Utilities|Array|RemoveItem (Variables|Default|GetPickup/Array) (CallFunction|GetCurrentpickup)))