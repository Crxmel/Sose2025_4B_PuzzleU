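; BP_Drehdingsdings is a rotatable piece that reports which of its eight symbol sides faces up.
; GetSymbol divides the world roll by 45 degrees, rounds it and selects the matching ESymbol value from indices 0 to 7, with no wrapping for negative roll.
; It also prints the roll on each call.
; An older float comparison using the AlmostEqual one-degree tolerance helper remains as unconnected, unused nodes.
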(fn GetSymbol
  (bind _returnvalue (Transformation|GetWorldRotation))
  ;[0.15 0.15 0.15 0.5] Zum identifiziren welche seite oben steht
  (Development|PrintString (Utilities|String|ToString(Float) (.roll _returnvalue)))
  (return (Utilities|Select :Index (Math|Float|Round (/ (.roll _returnvalue) 45.0)) :Option%200 "NewEnumerator0" :Option%201 "NewEnumerator1" :Option%202 "NewEnumerator2" :Option%203 "NewEnumerator3" :Option%204 "NewEnumerator4" :Option%205 "NewEnumerator5" :Option%206 "NewEnumerator6" :Option%207 "NewEnumerator7")))

(fn AlmostEqual
  (params (A :type Float%20%28double-precision%29) (B :type Float%20%28double-precision%29))
  (return (< (Math|Float|Absolute(Float) (- A B)) 1.0)))