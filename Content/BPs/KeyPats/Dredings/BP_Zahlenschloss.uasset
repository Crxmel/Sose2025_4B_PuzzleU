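; Combination lock puzzle with five rotating symbol dials, entered through the inherited Interact and left via exit input or a correct code.
; Left/right input cycles the selected dial with wraparound and marks it with an overlay highlight material.
; Up/down plays a shared Timeline that rolls the dial in 45-degree steps, blocking navigation until finished.
; Confirming compares each dial's GetSymbol result against the CorrectCode array; an older rotation-based check remains unconnected.
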(event Input|EnhancedActionEvents|EnhancedInputActionIA_ExitPuzzle
  (params (ActionValue :type Boolean) (ElapsedSeconds :type Float%20%28double-precision%29) (TriggeredSeconds :type Float%20%28double-precision%29) (InputAction :type Input%20Action%20Object%20Reference :default "/Game/Input/IA_Puzzle/IA_ExitPuzzle.IA_ExitPuzzle"))
  (CallFunction|ReturntoCharacter)
  (CallFunction|UpdateActiveButtonforHighlight false))

(event Input|EnhancedActionEvents|EnhancedInputActionIA_Navigate_Right
  (params (ActionValue :type Boolean) (ElapsedSeconds :type Float%20%28double-precision%29) (TriggeredSeconds :type Float%20%28double-precision%29) (InputAction :type Input%20Action%20Object%20Reference :default "/Game/Input/IA_Puzzle/IA_Navigate_Right.IA_Navigate_Right"))
  ;[0.05408 0.05352 0.15 0.5] Rechts
  ;;[0.3516 0 0 0.5] Input Block
  (if (not (Variables|Default|GetInputBlock))
    ;;[0 0.1874 0.2422 0.5] HighliteColor desselect
    (CallFunction|UpdateActiveButtonforHighlight false)
    ;;[0.15 0.15 0.15 0.5] next button count
    (Variables|Default|SetCorrectButtonIndex (+ (Variables|Default|GetCorrectButtonIndex) 1))
    ;;[0 0.7076 0.8385 0.5] HighliteColor select
    (Utilities|FlowControl|Sequence
      (:then_0
        ;;[0.3307 0.2835 0 0.5] Rotation vom neuen selecten button speichern
        (Variables|Default|SetZwischenspeicherRotation (.roll (Variables|/Script/Engine.SceneComponent|GetRelativeRotation (CallFunction|GetActiveButton))))
        ;;[0.15 0.15 0.15 0.5] Button select last
        (if (> (Variables|Default|GetCorrectButtonIndex) (Utilities|Array|LastIndex (Variables|Default|GetSelecctedDrehDings)))
          (Variables|Default|SetCorrectButtonIndex 0)))
      (:then_1
        (CallFunction|UpdateActiveButtonforHighlight true)))))

(event Input|EnhancedActionEvents|EnhancedInputActionIA_Navigate_Left
  (params (ActionValue :type Boolean) (ElapsedSeconds :type Float%20%28double-precision%29) (TriggeredSeconds :type Float%20%28double-precision%29) (InputAction :type Input%20Action%20Object%20Reference :default "/Game/Input/IA_Puzzle/IA_Navigate_Left.IA_Navigate_Left"))
  ;[0.15 0.05 0.05 0.5] Links
  ;;[0.3516 0 0 0.5] Input Block
  (if (not (Variables|Default|GetInputBlock))
    ;;[0 0.1874 0.2422 0.5] HighliteColor desselect
    (CallFunction|UpdateActiveButtonforHighlight false)
    ;;[0.15 0.15 0.15 0.5] next button count
    (Variables|Default|SetCorrectButtonIndex (- (Variables|Default|GetCorrectButtonIndex) 1))
    ;;[0 0.7076 0.8385 0.5] HighliteColor select
    (Utilities|FlowControl|Sequence
      (:then_0
        ;;[0.3307 0.2835 0 0.5] Rotation vom neuen selecten button speichern
        (Variables|Default|SetZwischenspeicherRotation (.roll (Variables|/Script/Engine.SceneComponent|GetRelativeRotation (CallFunction|GetActiveButton))))
        ;;[0.15 0.15 0.15 0.5] Button select last
        (if (< (Variables|Default|GetCorrectButtonIndex) 0)
          (Variables|Default|SetCorrectButtonIndex (Utilities|Array|LastIndex (Variables|Default|GetSelecctedDrehDings)))))
      (:then_1
        (CallFunction|UpdateActiveButtonforHighlight true)))))

(event Input|EnhancedActionEvents|EnhancedInputActionIA_Navigate_Down
  (params (ActionValue :type Boolean) (ElapsedSeconds :type Float%20%28double-precision%29) (TriggeredSeconds :type Float%20%28double-precision%29) (InputAction :type Input%20Action%20Object%20Reference :default "/Game/Input/IA_Puzzle/IA_Navigate_Down.IA_Navigate_Down"))
  ;[0.15 0.15 0.15 0.5] Rauf/Runter Rotation
  ;;[0.15 0.15 0.15 0.5] Input blockirt
  (if (not (Variables|Default|GetInputBlock))
    ;;[0.15 0.15 0.15 0.5] Input bloch an
    (Variables|Default|SetInputBlock (not (Variables|Default|GetInputBlock)))
    (Variables|Default|SetRauf/RunterTrigger 1.0)
    (bind _dreung (Timeline|Timeline PlayFromStart)
      (:Update
        (Transformation|SetRelativeRotation (CallFunction|GetActiveButton) (Math|Rotator|MakeRotator (+ (* (* _dreung (Variables|Default|GetRauf/RunterTrigger)) 45.0) (Variables|Default|GetZwischenspeicherRotation)) 0.0 0.0) false false))
      (:Finished
        (Variables|Default|SetZwischenspeicherRotation (.roll (Variables|/Script/Engine.SceneComponent|GetRelativeRotation (CallFunction|GetActiveButton))))
        ;;[0.15 0.15 0.15 0.5] InputBlock aus
        (Variables|Default|SetInputBlock false)))))

(event Input|EnhancedActionEvents|EnhancedInputActionIA_Navigate_UP
  (params (ActionValue :type Boolean) (ElapsedSeconds :type Float%20%28double-precision%29) (TriggeredSeconds :type Float%20%28double-precision%29) (InputAction :type Input%20Action%20Object%20Reference :default "/Game/Input/IA_Puzzle/IA_Navigate_UP.IA_Navigate_UP"))
  ;[0.15 0.15 0.15 0.5] Rauf/Runter Rotation
  ;;[0.15 0.15 0.15 0.5] Input blockirt
  (if (not (Variables|Default|GetInputBlock))
    ;;[0.15 0.15 0.15 0.5] Input bloch an
    (Variables|Default|SetInputBlock (not (Variables|Default|GetInputBlock)))
    (Variables|Default|SetRauf/RunterTrigger -1.0)
    (bind _dreung (Timeline|Timeline PlayFromStart)
      (:Update
        (Transformation|SetRelativeRotation (CallFunction|GetActiveButton) (Math|Rotator|MakeRotator (+ (* (* _dreung (Variables|Default|GetRauf/RunterTrigger)) 45.0) (Variables|Default|GetZwischenspeicherRotation)) 0.0 0.0) false false))
      (:Finished
        (Variables|Default|SetZwischenspeicherRotation (.roll (Variables|/Script/Engine.SceneComponent|GetRelativeRotation (CallFunction|GetActiveButton))))
        ;;[0.15 0.15 0.15 0.5] InputBlock aus
        (Variables|Default|SetInputBlock false)))))

(event Input|EnhancedActionEvents|EnhancedInputActionIA_Interact
  (params (ActionValue :type Boolean) (ElapsedSeconds :type Float%20%28double-precision%29) (TriggeredSeconds :type Float%20%28double-precision%29) (InputAction :type Input%20Action%20Object%20Reference :default "/Game/Input/IA_Interact.IA_Interact"))
  ;[0.15 0.15 0.15 0.5] Controlle bessere version
  (if (CallFunction|IsCodeCorrect)
    (CallFunction|ReturntoCharacter)
    (CallFunction|UpdateActiveButtonforHighlight false)))

(event EventBeginPlay
  ;[0.15 0.15 0.15 0.5] set ButtonArray
  (Variables|Default|SetSelecctedDrehDings (Utilities|Array|MakeArray (Variables|Default|GetDrehdingsdings_01) (Variables|Default|GetDrehdingsdings_02) (Variables|Default|GetDrehdingsdings_03) (Variables|Default|GetDrehdingsdings_04) (Variables|Default|GetDrehdingsdings_05))))

(fn ConstructionScript
  (|CallParentFunction))

(fn GetActiveButton
  (return (Utilities|Array|Get(acopy) (Variables|Default|GetSelecctedDrehDings) (Variables|Default|GetCorrectButtonIndex))))

(fn UpdateActiveButtonforHighlight
  (params (Selected :type Boolean))
  (Rendering|Material|SetOverlayMaterial (CallFunction|GetActiveButton) (select Selected "/Game/Material/NewFolder/MI_MaterialButtonHighlight.MI_MaterialButtonHighlight" 0) :!class /Script/Engine.MeshComponent))

(fn DoAnimationInputBlockFunktion
  (if (not (Variables|Default|GetInputBlock))
    (Variables|Default|SetInputBlock (not (Variables|Default|GetInputBlock)))
    (return)))

(fn IsCodeCorrect
  ;[0.15 0.15 0.15 0.5] wenn der loob nicht von der anderen returnnode abgebrochen wurde complitet er mir code richtig
  (for (_array_element _array_index) (Variables|Default|GetSelecctedDrehDings)
    ;[0.15 0.15 0.15 0.5] controllirt ob der code richtig ist indem der den ricchtigen code vom ESymbol (Enum) vergleicht
    (if (not (Utilities|Enum|Equal(Enum) (Default|GetSymbol _array_element) (Utilities|Array|Get(acopy) (Variables|Default|GetCorrectCode) _array_index)))
      ;[0.15 0.15 0.15 0.5] sobald es getriggerd wird wird es abgebrochen
      (return false)))
  (return true))

(fn Interact
  (params (PlayerCharacter :type BP%20Character%20Object%20Reference) (Pickup :type BP%20Pickup%20Actor%20Object%20Reference))
  (|CallParentFunction PlayerCharacter 0)
  (CallFunction|UpdateActiveButtonforHighlight true))