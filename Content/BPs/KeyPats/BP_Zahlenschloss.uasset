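; Combination lock puzzle ("Zahlenschloss") with five rotatable dials that the player operates after interacting with it.
; Left/right input cycles the selected dial with wraparound and an overlay highlight, while up/down rolls it in 45-degree steps.
; The interact input checks each dial in order for zero world roll, but only prints debug numbers, with no unlock action.
; A separate exit input returns control to the character.
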(event Input|EnhancedActionEvents|EnhancedInputActionIA_ExitPuzzle
  (params (ActionValue :type Boolean) (ElapsedSeconds :type Float%20%28double-precision%29) (TriggeredSeconds :type Float%20%28double-precision%29) (InputAction :type Input%20Action%20Object%20Reference :default "/Game/Input/IA_Puzzle/IA_ExitPuzzle.IA_ExitPuzzle"))
  (CallFunction|ReturntoCharacter))

(event Input|EnhancedActionEvents|EnhancedInputActionIA_Navigate_Right
  (params (ActionValue :type Boolean) (ElapsedSeconds :type Float%20%28double-precision%29) (TriggeredSeconds :type Float%20%28double-precision%29) (InputAction :type Input%20Action%20Object%20Reference :default "/Game/Input/IA_Puzzle/IA_Navigate_Right.IA_Navigate_Right"))
  (CallFunction|UpdateActiveButtonforHighlight false)
  (Variables|Default|SetCorrectButtonIndex (+ (Variables|Default|GetCorrectButtonIndex) 1))
  (Utilities|FlowControl|Sequence
    (:then_0
      (if (> (Variables|Default|GetCorrectButtonIndex) (Utilities|Array|LastIndex (Variables|Default|GetSelecctedDrehDings)))
        (Variables|Default|SetCorrectButtonIndex 0)))
    (:then_1
      (CallFunction|UpdateActiveButtonforHighlight true))))

(event Input|EnhancedActionEvents|EnhancedInputActionIA_Navigate_Left
  (params (ActionValue :type Boolean) (ElapsedSeconds :type Float%20%28double-precision%29) (TriggeredSeconds :type Float%20%28double-precision%29) (InputAction :type Input%20Action%20Object%20Reference :default "/Game/Input/IA_Puzzle/IA_Navigate_Left.IA_Navigate_Left"))
  (CallFunction|UpdateActiveButtonforHighlight false)
  (Variables|Default|SetCorrectButtonIndex (- (Variables|Default|GetCorrectButtonIndex) 1))
  (Utilities|FlowControl|Sequence
    (:then_0
      (if (< (Variables|Default|GetCorrectButtonIndex) 0)
        (Variables|Default|SetCorrectButtonIndex (Utilities|Array|LastIndex (Variables|Default|GetSelecctedDrehDings)))))
    (:then_1
      (CallFunction|UpdateActiveButtonforHighlight true))))

(event Input|EnhancedActionEvents|EnhancedInputActionIA_Navigate_Down
  (params (ActionValue :type Boolean) (ElapsedSeconds :type Float%20%28double-precision%29) (TriggeredSeconds :type Float%20%28double-precision%29) (InputAction :type Input%20Action%20Object%20Reference :default "/Game/Input/IA_Puzzle/IA_Navigate_Down.IA_Navigate_Down"))
  (CallFunction|RotateActiveButton 1.0)
  (Development|PrintString (Utilities|String|ToString(Float) (.roll (Transformation|GetWorldRotation (CallFunction|GetActiveButton))))))

(event Input|EnhancedActionEvents|EnhancedInputActionIA_Navigate_UP
  (params (ActionValue :type Boolean) (ElapsedSeconds :type Float%20%28double-precision%29) (TriggeredSeconds :type Float%20%28double-precision%29) (InputAction :type Input%20Action%20Object%20Reference :default "/Game/Input/IA_Puzzle/IA_Navigate_UP.IA_Navigate_UP"))
  (CallFunction|RotateActiveButton -1.0)
  (Development|PrintString (Utilities|String|ToString(Float) (.roll (Transformation|GetWorldRotation (CallFunction|GetActiveButton))))))

(event Input|EnhancedActionEvents|EnhancedInputActionIA_Interact
  (params (ActionValue :type Boolean) (ElapsedSeconds :type Float%20%28double-precision%29) (TriggeredSeconds :type Float%20%28double-precision%29) (InputAction :type Input%20Action%20Object%20Reference :default "/Game/Input/IA_Interact.IA_Interact"))
  (if (== (.roll (Transformation|GetWorldRotation (Variables|Default|GetDrehdingsdings_01))) 0.0)
    (Development|PrintString "1")
    (if (== (.roll (Transformation|GetWorldRotation (Variables|Default|GetDrehdingsdings_02))) 0.0)
      (Development|PrintString "2")
      (if (== (.roll (Transformation|GetWorldRotation (Variables|Default|GetDrehdingsdings_03))) 0.0)
        (Development|PrintString "3")
        (if (== (.roll (Transformation|GetWorldRotation (Variables|Default|GetDrehdingsdings_04))) 0.0)
          (Development|PrintString "4")
          (if (== (.roll (Transformation|GetWorldRotation (Variables|Default|GetDrehdingsdings_05))) 0.0)
            (Development|PrintString "5")))))))

(event EventInteract
  (params (PlayerCharacter :type BP%20Character%20Object%20Reference))
  (|CallParentFunction PlayerCharacter)
  (CallFunction|UpdateActiveButtonforHighlight true))

(event EventBeginPlay
  (Variables|Default|SetSelecctedDrehDings (Utilities|Array|MakeArray (Variables|Default|GetDrehdingsdings_01) (Variables|Default|GetDrehdingsdings_02) (Variables|Default|GetDrehdingsdings_03) (Variables|Default|GetDrehdingsdings_04) (Variables|Default|GetDrehdingsdings_05))))

(fn ConstructionScript
  (|CallParentFunction))

(fn GetActiveButton
  (return (Utilities|Array|Get(acopy) (Variables|Default|GetSelecctedDrehDings) (Variables|Default|GetCorrectButtonIndex))))

(fn UpdateActiveButtonforHighlight
  (params (Selected :type Boolean))
  (Rendering|Material|SetOverlayMaterial (CallFunction|GetActiveButton) (select Selected "/Game/Material/NewFolder/MI_MaterialButtonHighlight.MI_MaterialButtonHighlight" 0) :!class /Script/Engine.MeshComponent))

(fn RotateActiveButton
  (params (B :type Float%20%28double-precision%29))
  (bind _output (CallFunction|GetActiveButton))
  (Transformation|SetRelativeRotation _output (Math|Rotator|MakeRotator (+ (.roll (Variables|/Script/Engine.SceneComponent|GetRelativeRotation _output)) (* 45.0 B)) 0.0 0.0) false false))