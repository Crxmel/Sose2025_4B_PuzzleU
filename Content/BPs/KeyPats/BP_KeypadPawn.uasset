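; Keypad puzzle pawn where the player enters a code on a twelve-button pad after interacting with it.
; Directional input moves a wrapping index through the button array in a three-column layout, highlighting the selection with an overlay material.
; Interact appends the selected label to the Code text, capped at CorrectCode's length.
; ButtonBack checks the code, returning to the character or clearing on failure, while ButtonEnter clears the display.
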(event Input|EnhancedActionEvents|EnhancedInputActionIA_ExitPuzzle
  (params (ActionValue :type Boolean) (ElapsedSeconds :type Float%20%28double-precision%29) (TriggeredSeconds :type Float%20%28double-precision%29) (InputAction :type Input%20Action%20Object%20Reference :default "/Game/Input/IA_Puzzle/IA_ExitPuzzle.IA_ExitPuzzle"))
  ;[0.15 0.15 0.15 0.5] Prosses AnPosess
  (CallFunction|ReturntoCharacter))

(event Input|EnhancedActionEvents|EnhancedInputActionIA_Navigate_Right
  (params (ActionValue :type Boolean) (ElapsedSeconds :type Float%20%28double-precision%29) (TriggeredSeconds :type Float%20%28double-precision%29) (InputAction :type Input%20Action%20Object%20Reference :default "/Game/Input/IA_Puzzle/IA_Navigate_Right.IA_Navigate_Right"))
  (CallFunction|NavigateButtons 1))

(event Input|EnhancedActionEvents|EnhancedInputActionIA_Navigate_Left
  (params (ActionValue :type Boolean) (ElapsedSeconds :type Float%20%28double-precision%29) (TriggeredSeconds :type Float%20%28double-precision%29) (InputAction :type Input%20Action%20Object%20Reference :default "/Game/Input/IA_Puzzle/IA_Navigate_Left.IA_Navigate_Left"))
  (CallFunction|NavigateButtons -1))

(event Input|EnhancedActionEvents|EnhancedInputActionIA_Navigate_Down
  (params (ActionValue :type Boolean) (ElapsedSeconds :type Float%20%28double-precision%29) (TriggeredSeconds :type Float%20%28double-precision%29) (InputAction :type Input%20Action%20Object%20Reference :default "/Game/Input/IA_Puzzle/IA_Navigate_Down.IA_Navigate_Down"))
  (CallFunction|NavigateButtons 3))

(event Input|EnhancedActionEvents|EnhancedInputActionIA_Navigate_UP
  (params (ActionValue :type Boolean) (ElapsedSeconds :type Float%20%28double-precision%29) (TriggeredSeconds :type Float%20%28double-precision%29) (InputAction :type Input%20Action%20Object%20Reference :default "/Game/Input/IA_Puzzle/IA_Navigate_UP.IA_Navigate_UP"))
  (CallFunction|NavigateButtons -3))

(event Input|EnhancedActionEvents|EnhancedInputActionIA_Interact
  (params (ActionValue :type Boolean) (ElapsedSeconds :type Float%20%28double-precision%29) (TriggeredSeconds :type Float%20%28double-precision%29) (InputAction :type Input%20Action%20Object%20Reference :default "/Game/Input/IA_Interact.IA_Interact"))
  (if (== (CallFunction|GetSelectedButton) (Variables|Default|GetButton_Back))
    ;[0.15 0.15 0.15 0.5] checking code ob richtig
    (if (CallFunction|IsCodeCorrect)
      (CallFunction|ReturntoCharacter)
      (Development|PrintString "Richtig" true true "(R=0.099708,G=1.000000,B=0.000000,A=1.000000)" 5.0)
      (else
        (CallFunction|ClearDisplay)
        (Development|PrintString "Falsch" true true "(R=0.000000,G=0.660000,B=1.000000,A=1.000000)" 5.0)))
    (elif (== (CallFunction|GetSelectedButton) (Variables|Default|GetButton_Enter))
      (CallFunction|ClearDisplay)
      (elif (not (CallFunction|IsCodeCompied))
        (CallFunction|AddtoDisplay (Variables|/Game/BPs/KeyPats/BP_Button.BP_Button_C|GetButtonLable (CallFunction|GetSelectedButton)))))))

(event EventInteract
  (params (PlayerCharacter :type BP%20Character%20Object%20Reference))
  ;[0.15 0.15 0.15 0.5] Prosses AnPosess
  (|CallParentFunction PlayerCharacter)
  (CallFunction|UpdateHiglithOfSelectedButton true))

(event EventReturntoCharacter
  ;[0.15 0.15 0.15 0.5] Prosses AnPosess
  ;;[0.15 0.15 0.15 0.5] Zum unhiglighte
  (|CallParentFunction)
  (CallFunction|UpdateHiglithOfSelectedButton false))

(event EventBeginPlay
  (Variables|Default|SetButtonArray (Utilities|Array|MakeArray (Variables|Default|GetButton_1) (Variables|Default|GetButton_2) (Variables|Default|GetButton_3) (Variables|Default|GetButton_4) (Variables|Default|GetButton_5) (Variables|Default|GetButton_6) (Variables|Default|GetButton_7) (Variables|Default|GetButton_8) (Variables|Default|GetButton_9) (Variables|Default|GetButton_Back) (Variables|Default|GetButton_0) (Variables|Default|GetButton_Enter)))
  (CallFunction|ClearDisplay))

(fn ConstructionScript)

(fn GetSelectedButton
  (return (Utilities|Array|Get(acopy) (Variables|Default|GetButtonArray) (Variables|Default|GetCorrectButtenIndex))))

(fn UpdateHiglithOfSelectedButton
  (params (Select :type Boolean))
  (Rendering|Material|SetOverlayMaterial (CallFunction|GetSelectedButton) (select Select "/Game/Material/NewFolder/MI_MaterialButtonHighlight.MI_MaterialButtonHighlight" 0) :!class /Script/Engine.MeshComponent))

(fn NavigateButtons
  (params (Derection :type Integer))
  (CallFunction|UpdateHiglithOfSelectedButton false)
  (Variables|Default|SetCorrectButtenIndex (+ (Variables|Default|GetCorrectButtenIndex) Derection))
  (Utilities|FlowControl|Sequence
    (:then_0
      (if (> (Variables|Default|GetCorrectButtenIndex) (Utilities|Array|LastIndex (Variables|Default|GetButtonArray)))
        (Variables|Default|SetCorrectButtenIndex (- (Variables|Default|GetCorrectButtenIndex) (Utilities|Array|Length (Variables|Default|GetButtonArray))))))
    (:then_1
      (if (< (Variables|Default|GetCorrectButtenIndex) 0)
        (Variables|Default|SetCorrectButtenIndex (+ (Variables|Default|GetCorrectButtenIndex) (Utilities|Array|Length (Variables|Default|GetButtonArray))))))
    (:then_2
      (CallFunction|UpdateHiglithOfSelectedButton true))))

(fn ClearDisplay
  (Rendering|Components|TextRender|SetText (Variables|Default|GetCode) (Utilities|Text|ToText(String) "")))

(fn AddtoDisplay
  (params (Text :type String))
  (bind _code (Variables|Default|GetCode))
  (Rendering|Components|TextRender|SetText _code (Utilities|Text|ToText(String) (Utilities|String|Append (Utilities|String|ToString(Text) (Variables|/Script/Engine.TextRenderComponent|GetText _code)) Text))))

(fn IsCodeCompied
  (return (== (Utilities|String|Len (Utilities|String|ToString(Text) (Variables|/Script/Engine.TextRenderComponent|GetText (Variables|Default|GetCode)))) (Utilities|String|Len (Variables|Default|GetCorrectCode)))))

(fn IsCodeCorrect
  (return (Utilities|Enum|Equal(Enum) (Utilities|String|ToString(Text) (Variables|/Script/Engine.TextRenderComponent|GetText (Variables|Default|GetCode))) (Variables|Default|GetCorrectCode))))