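; Base interactable pawn that the player can possess, apparently for puzzles, and later leave to return to the character.
; Interact stores the character and, if allowed, blends the view to itself, delays, possesses it and swaps character input mapping for puzzle mapping.
; ReturnToCharacter reverses this after repositioning the character via a downward trace from the camera to stand on the surface below.
; Child classes must supply a CameraComponent for that repositioning.
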(event Custom|GetPossessed
  (bind _returnvalue (Game|GetPlayerController 0))
  (bind _returnvalue_2 (PlayerController|LocalPlayerSubsystems|GetEnhancedInputLocalPlayerSubsystem _returnvalue))
  ;[0.15 0.15 0.15 0.5] Get Possesed
  (Input|RemoveMappingContext _returnvalue_2 (Variables|Default|GetCharacterMapping%20Context) "(bIgnoreAllPressedKeysUntilRelease=True,bForceImmediately=False,bNotifyUserSettings=False)")
  (Game|Player|SetViewTargetwithBlend (Game|GetPlayerController 0) self (Variables|Default|GetSmoothProssessDoration) "VTBlend_Linear" 0.0 false)
  (Utilities|FlowControl|Delay (Variables|Default|GetSmoothProssessDoration))
  (Pawn|Possess (Game|GetPlayerController 0) self)
  (Input|AddMappingContext _returnvalue_2 (Variables|Default|GetPuzzleMapping%20Context) 0 "(bIgnoreAllPressedKeysUntilRelease=True,bForceImmediately=False,bNotifyUserSettings=False)"))

(event Custom|ReturnToCharacter
  (bind _returnvalue (Game|GetPlayerController 0))
  (bind _returnvalue_2 (PlayerController|LocalPlayerSubsystems|GetEnhancedInputLocalPlayerSubsystem _returnvalue))
  ;[0.15 0.15 0.15 0.5] Possess Character
  (CallFunction|PositionPlayerCharacter)
  (Input|RemoveMappingContext _returnvalue_2 (Variables|Default|GetPuzzleMapping%20Context) "(bIgnoreAllPressedKeysUntilRelease=True,bForceImmediately=False,bNotifyUserSettings=False)")
  (Game|Player|SetViewTargetwithBlend (Game|GetPlayerController 0) (Variables|Default|GetPlayer%20Character) (Variables|Default|GetSmoothProssessDoration) "VTBlend_Linear" 0.0 false)
  (Utilities|FlowControl|Delay (Variables|Default|GetSmoothProssessDoration))
  (Pawn|Possess (Game|GetPlayerController 0) (Variables|Default|GetPlayer%20Character))
  (Input|AddMappingContext _returnvalue_2 (Variables|Default|GetCharacterMapping%20Context) 0 "(bIgnoreAllPressedKeysUntilRelease=True,bForceImmediately=False,bNotifyUserSettings=False)"))

(event EventInteract
  (params (PlayerCharacter :type BP%20Character%20Object%20Reference))
  ;[0.15 0.15 0.15 0.5] get interactable with
  (Variables|Default|SetPlayer%20Character PlayerCharacter)
  (if (Variables|Default|GetCanBeProsses)
    (CallFunction|GetPossessed)))

(fn ConstructionScript)

(fn PositionPlayerCharacter
  (bind _output_get (LocalVariables|SetCam (Actor|GetComponentbyClass "/Script/Engine.CameraComponent")))
  (Utilities|IsValid _output_get
    (:Is%20Valid
      (Transformation|SetActorLocation (Variables|Default|GetPlayer%20Character) (Math|Vector|MakeVector 0.0 0.0 (.z (Transformation|GetWorldLocation (LocalVariables|GetCam)))) false false)
      (bind (_outhit _returnvalue) (Collision|LineTraceForObjects (Transformation|GetWorldLocation (LocalVariables|GetCam)) (- (Transformation|GetWorldLocation (LocalVariables|GetCam)) "0.000000,0.000000,600.000000") (Utilities|Array|MakeArray "ObjectTypeQuery1" "ObjectTypeQuery2") false 0 "ForDuration" true "(R=1.000000,G=0.000000,B=0.000000,A=1.000000)" "(R=0.000000,G=1.000000,B=0.000000,A=1.000000)" 1e+01))
      (if _returnvalue
        (Transformation|SetActorLocation (Variables|Default|GetPlayer%20Character) (+ (.Location (Collision|BreakHitResult _outhit)) (Math|Vector|MakeVector 0.0 0.0 (+ (Variables|/Script/Engine.CapsuleComponent|GetCapsuleHalfHeight (Variables|/Script/Engine.Character|GetCapsuleComponent (Variables|Default|GetPlayer%20Character))) 1.0))) false false)))
    (:Is%20Not%20Valid
      (Development|PrintString "BP_InteractableProssessable child braucht cameracomponent konnte aber nix finden" true true "(R=0.000000,G=0.660000,B=1.000000,A=1.000000)" 5.0))))