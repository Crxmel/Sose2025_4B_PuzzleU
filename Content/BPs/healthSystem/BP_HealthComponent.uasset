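; BP_HealthComponent is a health component that tracks current health and signals when its owner dies.
; Current health starts at MaxHealth on BeginPlay, and the TakeDamage event subtracts the damage amount from it without clamping.
; When the depletion check finds health at or below zero, Die calls OnDeath, with no guard against repeat calls on further damage.
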(event Custom|TakeDamage
  (params (DamageAmaunt :type Float%20%28double-precision%29))
  (Variables|Default|SetCurrentHelth (- (Variables|Default|GetCurrentHelth) DamageAmaunt))
  (if (CallFunction|IsHealthDepidet)
    (CallFunction|Die)))

(event Custom|Die
  (Default|CallOnDeath))

(event EventBeginPlay
  (Variables|Default|SetCurrentHelth (Variables|Default|GetMaxHealth)))

(fn IsHealthDepidet
  (return (<= (Variables|Default|GetCurrentHelth) 0.0)))