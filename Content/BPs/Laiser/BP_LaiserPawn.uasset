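; BP_LaiserPawn is a rotatable laser puzzle pawn that acts as a beam source or redirector, with yaw input and an exit back to the character.
; Sources line-trace every tick, set the Niagara beam's length and notify any laser pawn hit.
; A Box hit fires CallHitByLaiser and, if redirection is allowed, re-emits.
; A last-hit timestamp limits this to once per frame and switches off unlit non-source beams.
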(event Custom|GetHitByLaiser
  (params (HitComponent :type Primitive%20Component%20Object%20Reference))
  (if (== HitComponent (Variables|Default|GetBox))
    (if (CallFunction|TimeHasPassedSinceLastHit)
      (Variables|Default|SetLastHitTime (Utilities|Time|GetGameTimeinSeconds))
      (Default|CallHitbyLaiser)
      (if (Variables|Default|GetCanRederectLight)
        (CallFunction|SetVFXEnabled true)
        (CallFunction|EmitLaiser)))))

(event Input|EnhancedActionEvents|EnhancedInputActionIA_Mous
  (params (ActionValue :type Vector%202D%20Structure) (ElapsedSeconds :type Float%20%28double-precision%29) (TriggeredSeconds :type Float%20%28double-precision%29) (InputAction :type Input%20Action%20Object%20Reference :default "/Game/Input/IA/IA_Mous.IA_Mous"))
  (Transformation|AddActorLocalRotation (Math|Rotator|MakeRotator 0.0 0.0 (* (.x ActionValue) (Utilities|Time|GetWorldDeltaSeconds) (Variables|Default|GetRotationSpeed))) false false))

(event Input|EnhancedActionEvents|EnhancedInputActionIA_ExitPuzzle
  (params (ActionValue :type Boolean) (ElapsedSeconds :type Float%20%28double-precision%29) (TriggeredSeconds :type Float%20%28double-precision%29) (InputAction :type Input%20Action%20Object%20Reference :default "/Game/Input/IA_Puzzle/IA_ExitPuzzle.IA_ExitPuzzle"))
  (CallFunction|ReturntoCharacter))

(event EventTick
  (params (DeltaSeconds :type Float%20%28single-precision%29))
  (if (Variables|Default|GetIsLaiserSource)
    (CallFunction|EmitLaiser)
    (elif (CallFunction|TimeHasPassedSinceLastHit)
      (CallFunction|SetVFXEnabled false))))

(event EventBeginPlay
  (CallFunction|SetVFXEnabled (Variables|Default|GetIsLaiserSource)))

(fn ConstructionScript
  (|CallParentFunction)
  (CallFunction|SetVFXEnabled (Variables|Default|GetIsLaiserSource)))

(fn CheckforLaisetHit
  (bind _laiserorigen (Variables|Default|GetLaiserOrigen))
  (bind _returnvalue (Transformation|GetWorldLocation _laiserorigen))
  (bind (_outhit _returnvalue_2) (Collision|LineTraceForObjects _returnvalue (+ _returnvalue (* (Math|Vector|GetForwardVector _laiserorigen) (Variables|Default|GetMaxLaiserRange))) (Utilities|Array|MakeArray "ObjectTypeQuery1" "ObjectTypeQuery2" "ObjectTypeQuery3" "ObjectTypeQuery4") false 0 "ForOneFrame"))
  (if _returnvalue_2
    (bind _asbp_laiser_pawn (Utilities|Casting|CastToBP_LaiserPawn (.HitActor (Collision|BreakHitResult _outhit))))
    (return true (Math|Vector|VectorLength (- (.ImpactPoint (Collision|BreakHitResult _outhit)) (Transformation|GetWorldLocation (Variables|Default|GetLaiserOrigen)))) _asbp_laiser_pawn (.HitComponent (Collision|BreakHitResult _outhit)))
    (else
      (return false 0.0 0 0))))

(fn SetVFXEnabled
  (params (IsEnabled :type Boolean))
  (bind _ns_beam (Variables|Default|GetNS_Beam))
  (if IsEnabled
    (Components|Activation|Activate _ns_beam false)
    (else
      (Components|Activation|Deactivate _ns_beam))))

(fn EmitLaiser
  (bind (_hitsompfing _distancetohit _hitlaisercomponent _hitcomponent) (CallFunction|CheckforLaisetHit))
  (if _hitsompfing
    (Niagara|SetNiagaraVariable(Float) (Variables|Default|GetNS_Beam) "LaiserLenght" _distancetohit)
    (Utilities|IsValid _hitlaisercomponent
      (:Is%20Valid
        (CallFunction|GetHitbyLaiser _hitlaisercomponent _hitcomponent)))))

(fn TimeHasPassedSinceLastHit
  (return (> (Utilities|Time|GetGameTimeinSeconds) (Variables|Default|GetLastHitTime))))