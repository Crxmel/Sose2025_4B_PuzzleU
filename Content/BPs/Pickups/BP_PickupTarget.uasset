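; BP_PickupTarget is an interactable target that either rotates or receives a pickup of a desired class.
; When its NewVar flag is true, Interact turns the root by a fixed 45-degree relative step.
; Otherwise, it validates the pickup, requires an exact class match with DesierPickup, attaches it to the Scene component through PrepareForHoldingAAttatchTo, and sets and returns NewVar as false.
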(fn ConstructionScript)

(fn Rotate
  (Transformation|AddRelativeRotation (Variables|Default|GetDefaultSceneRoot) "0.000000,45.000000,0.000000" false false))

(fn Interact
  (params (PlayerCharacter :type BP%20Character%20Object%20Reference) (Pickup :type BP%20Pickup%20Actor%20Object%20Reference))
  (if (Variables|Default|GetNewVar)
    (CallFunction|Rotate)
    (else
      (Utilities|IsValid Pickup
        (:Is%20Valid
          (if (== (Utilities|GetClass Pickup) (Variables|Default|GetDesier%20pickup))
            ;[0.15 0.15 0.15 0.5] Attatch to
            (Default|PrepareforHoldingAAttatchto Pickup (Variables|Default|GetScene))
            (bind _output_get (Variables|Default|SetNewVar false))
            (return _output_get)))))))