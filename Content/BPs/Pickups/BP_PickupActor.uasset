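; BP_PickupActor is a physics-driven pickup that can be held and dropped.
; PrepareForHoldingAAttatchTo disables the static mesh's physics and collision, then attaches to the supplied component, snapping location and rotation while keeping world scale.
; Drop detaches with the world transform preserved, then restores query and physics collision and physics simulation.
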(event Custom|PrepareForHoldingAAttatchTo
  (params (component%20to%20attatch%20to :type Scene%20Component%20Object%20Reference))
  (Physics|SetSimulatePhysics (Variables|Default|GetStaticMesh) false)
  (Collision|SetCollisionEnabled (Variables|Default|GetStaticMesh) "NoCollision")
  (Transformation|AttachComponentToComponent component%20to%20attatch%20to "None" "SnapToTarget" "SnapToTarget" "KeepWorld" true))

(event Custom|Drop
  (Transformation|DetachFromActor "KeepWorld" "KeepWorld" "KeepWorld")
  (Collision|SetCollisionEnabled (Variables|Default|GetStaticMesh) "QueryAndPhysics")
  (Physics|SetSimulatePhysics (Variables|Default|GetStaticMesh) true))

(fn ConstructionScript)